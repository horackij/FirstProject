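; Player controller Blueprint that adds animated transitions to the pause menu supplied by its parent class.
; Displaying the menu calls the parent event, then plays the PauseMenu widget's animation forward.
; Removing it plays the same animation in reverse and waits a short fixed delay before calling the parent removal, so the transition can show first.
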(event EventBeginPlay)

(event EventTick
  (params (DeltaSeconds :type Float%20%28single-precision%29)))

(event EventDisplayPauseMenu
  (|CallParentFunction)
  (bind _aspause_menu (Utilities|Casting|CastToPauseMenu (Variables|Default|GetPauseMenu)))
  (UserInterface|Animation|PlayAnimation _aspause_menu (Variables|/Game/HUD/PauseMenu.PauseMenu_C|GetPauseMenuanimation _aspause_menu) 0.0 1 "Forward" 1.0))

(event EventRemovePauseMenu
  (bind _aspause_menu (Utilities|Casting|CastToPauseMenu (Variables|Default|GetPauseMenu)))
  (UserInterface|Animation|PlayAnimation _aspause_menu (Variables|/Game/HUD/PauseMenu.PauseMenu_C|GetPauseMenuanimation _aspause_menu) 0.0 1 "Reverse" 1.0)
  (Utilities|FlowControl|Delay 0.25)
  (|CallParentFunction))

(fn ConstructionScript)